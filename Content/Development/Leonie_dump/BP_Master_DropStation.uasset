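; BP_Master_DropStation is a base drop station where the player hands over items from the inventory.
; A range trigger tracks the player, and IA_Pickup toggles a lazily created WBP_DropUI showing the inventory, optionally pausing the game.
; Items passed to ReportDroppObjects are added to the station's dropped list and removed from BP_InventorySystem by name plus pickup time.
; OpenUIFromInput is a separate event so child Blueprints can override the opening behavior.
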(event `self.ReceiveBeginPlay`
  (`self.EnableInput` (`GameplayStatics.GetPlayerController` 0))
  (bind _outactors (`GameplayStatics.GetAllActorsOfClass` "/Game/Development/Leonie_dump/Inventory/BP_InventorySystem.BP_InventorySystem_C"))
  (set `self.InventorySystem_Ref` (`|GetArrayItem` _outactors)))

(event `self.RangeTrigger.OnComponentBeginOverlap`
  (params (OverlappedComponent :type "PrimitiveComponent Object Reference") (OtherActor :type "Actor Object Reference") (OtherComp :type "PrimitiveComponent Object Reference") (OtherBodyIndex :type Integer) (bFromSweep :type Boolean) (SweepResult :type "HitResult Structure (by ref)"))
  ;[1 1 1] Player Detection
  (cast `/Game/StarterContent/ThirdPerson/Blueprints/BP_ThirdPersonCharacter` OtherActor)
  (set `self.PlayerIsInRange` true))

(event `self.RangeTrigger.OnComponentEndOverlap`
  (params (OverlappedComponent :type "PrimitiveComponent Object Reference") (OtherActor :type "Actor Object Reference") (OtherComp :type "PrimitiveComponent Object Reference") (OtherBodyIndex :type Integer))
  ;[1 1 1] Player Detection
  (cast `/Game/StarterContent/ThirdPerson/Blueprints/BP_ThirdPersonCharacter` OtherActor)
  (set `self.PlayerIsInRange` false))

(event `EnhancedInput|/Game/Development/Leonie_dump/Levels_dump/IA_Pickup`
  (params (ActionValue :type Boolean) (ElapsedSeconds :type "Float (double-precision)") (TriggeredSeconds :type "Float (double-precision)") (InputAction :type "InputAction Object Reference" :default "/Game/Development/Leonie_dump/Levels_dump/IA_Pickup.IA_Pickup"))
  (:`Completed`
    (`self.OpenUIFromInput`)))

(event `OpenUIFromInput`
  ;[1 1 1] Open UI
  (if (`self.PlayerIsInRange`)
    (`self.OpenOrCloseDropUI`)))

(event `ReportDroppObjects`
  (params (Items :type "Array of /Game/Development/Leonie_dump/PickUps/ItemData Structure"))
  (`KismetArrayLibrary.Array_Clear` (`self.ReportedDroppedObjects_0`))
  (bind _output_get (set `self.ReportedDroppedObjects_0` Items))
  (`self.AddItemsToDroppedList` _output_get))

(fn `AddItemsToDroppedList`
  (params (ItemsToAdd :type "Array of /Game/Development/Leonie_dump/PickUps/ItemData Structure"))
  (for _array_element ItemsToAdd
    (`KismetArrayLibrary.Array_Add` (`self.AllDroppedObjects`) _array_element)
    (bind ((`Name_4_F8E0E59F4DED3ECE3D7832A06FFC4421` _name) (`PickupTime_23_72B68219414DE7AFB37B29B6206C8D61` _pickuptime)) (break `/Game/Development/Leonie_dump/PickUps/ItemData` _array_element))
    (`/Game/Development/Leonie_dump/Inventory/BP_InventorySystem.TryRemoveItem` (`self.InventorySystem_Ref`) (`KismetStringLibrary.Concat_StrStr` (`KismetTextLibrary.Conv_TextToString` _name) (`KismetStringLibrary.Conv_DoubleToString` _pickuptime)))
    (`KismetSystemLibrary.PrintString` "Added Item")))

(fn `OpenOrCloseDropUI`
  (bind _returnvalue (`GameplayStatics.GetPlayerController` 0))
  ;[1 1 1] On or off?
  (`/Engine/EditorBlueprintResources/StandardMacros.IsValid` (`self.WB_DropUI_Ref`)
    (:`Is Valid`
      (if (`Widget.IsVisible` (`self.WB_DropUI_Ref`))
        ;[1 1 1] Remove Widget
        (`GameplayStatics.SetGamePaused` false)
        (`Widget.RemoveFromParent` (`self.WB_DropUI_Ref`))
        (`WidgetBlueprintLibrary.SetInputMode_GameOnly` _returnvalue)
        (set `PlayerController.bShowMouseCursor` false _returnvalue)
        (else
          ;[1 1 1] Create WIdget
          (`UserWidget.AddToViewport` (stale _output_get) 0 :!label _label)
          (`WidgetBlueprintLibrary.SetInputMode_GameAndUIEx` (`GameplayStatics.GetPlayerController` 0) (`self.WB_DropUI_Ref`) "DoNotLock" false)
          (set `PlayerController.bShowMouseCursor` true (`GameplayStatics.GetPlayerController` 0))
          (if (`self.PauseGameWhileUIIsActive`)
            (`GameplayStatics.SetGamePaused` true))
          (`/Game/Development/Leonie_dump/Puzzles/WBP_DropUI.UpdateInventoryShowcase` (`self.WB_DropUI_Ref`) (`/Game/Development/Leonie_dump/Inventory/BP_InventorySystem.Inventory` (`self.InventorySystem_Ref`))))))
    (:`Is Not Valid`
      (bind _returnvalue_2 (`|CreateWidget` "/Game/Development/Leonie_dump/Puzzles/WBP_DropUI.WBP_DropUI_C" null self))
      (bind _output_get (set `self.WB_DropUI_Ref` _returnvalue_2))
      (goto _label))))

(fn `UpdateInventory`)

(fn `UserConstructionScript`)