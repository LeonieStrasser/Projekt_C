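; BP_SunRayRiddle is a time-of-day puzzle where the player must use a button while a moving sun ray hits its target.
; Tick lerps the ray endpoint and Niagara beam between morning and evening points using the survival manager's NightProgressValue.
; Overlap of the moving trigger with the target trigger arms and reveals the button zone.
; The player character entering the armed zone solves it once and makes the linked next puzzle appear.
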(event `self.ReceiveBeginPlay`
  ;[1 1 1] References
  (bind _outactors (`GameplayStatics.GetAllActorsOfClass` "/Game/Development/Fea_dump/BP_SurvivalManager.BP_SurvivalManager_C"))
  (set `self.SurvivalManager_Ref` (`|GetArrayItem` _outactors))
  ;[1 1 1] Set Visibility
  (`SceneComponent.SetVisibility` (`self.ButtonTriggerZone`) false false)
  (`SceneComponent.SetVisibility` (`self.Sphere1`) false false)
  (`SceneComponent.SetVisibility` (`self.Sphere`) false false)
  (`/Engine/EditorBlueprintResources/StandardMacros.IsValid` (`self.NextPuzzle`)
    (:`Is Not Valid`
      (`KismetSystemLibrary.PrintString` "Sun Ray Riddle has no Reference for Next Puzzle! LG Dr. Debug" true true (struct :`R` 1.0 :`B` 0.130888 :`A` 1.0) 20.0))))

(event `self.ReceiveTick`
  (params (DeltaSeconds :type "Float (single-precision)"))
  (bind _returnvalue (`KismetMathLibrary.VLerp` (`SceneComponent.K2_GetComponentLocation` (`self.MorningPoint`)) (`SceneComponent.K2_GetComponentLocation` (`self.EveningPoint`)) (`/Game/Development/Fea_dump/BP_SurvivalManager.night_progress_value` (`self.SurvivalManager_Ref`))))
  ;[1 1 1] Move Moving Ray Endpoint
  (`SceneComponent.K2_SetWorldLocation` (`self.MovingENdPoint`) _returnvalue false false)
  (`NiagaraComponent.SetVariableVec3` (`self.NS_RiddleRay`) "ENdLocation" _returnvalue))

(event `self.TargetTrigger.OnComponentBeginOverlap`
  (params (OverlappedComponent :type "PrimitiveComponent Object Reference") (OtherActor :type "Actor Object Reference") (OtherComp :type "PrimitiveComponent Object Reference") (OtherBodyIndex :type Integer) (bFromSweep :type Boolean) (SweepResult :type "HitResult Structure (by ref)"))
  ;[1 1 1] Button Avtivation and deavtivation per Ray
  (if (`self.ButtonWasActivated`)
    _
    (elif (== OtherComp (`self.MovingTrigger`))
      (set `self.ActivatorIsActive` true)
      (`SceneComponent.SetVisibility` (`self.ButtonTriggerZone`) true false))))

(event `self.TargetTrigger.OnComponentEndOverlap`
  (params (OverlappedComponent :type "PrimitiveComponent Object Reference") (OtherActor :type "Actor Object Reference") (OtherComp :type "PrimitiveComponent Object Reference") (OtherBodyIndex :type Integer))
  ;[1 1 1] Button Avtivation and deavtivation per Ray
  (if (`SceneComponent.IsVisible` (`self.ButtonTriggerZone`))
    (if (== OtherComp (`self.MovingTrigger`))
      (set `self.ActivatorIsActive` false)
      (`SceneComponent.SetVisibility` (`self.ButtonTriggerZone`) false false))))

(event `self.ButtonTriggerZone.OnComponentBeginOverlap`
  (params (OverlappedComponent :type "PrimitiveComponent Object Reference") (OtherActor :type "Actor Object Reference") (OtherComp :type "PrimitiveComponent Object Reference") (OtherBodyIndex :type Integer) (bFromSweep :type Boolean) (SweepResult :type "HitResult Structure (by ref)"))
  ;[1 1 1] Button Avtivation
  (if (`self.ActivatorIsActive`)
    (cast `/Game/StarterContent/ThirdPerson/Blueprints/BP_ThirdPersonCharacter` OtherActor)
    (`/Engine/EditorBlueprintResources/StandardMacros.DoOnce` false
      (:`Completed`
        (set `self.ButtonWasActivated` true)
        (`self.ReportPuzzleSolving`)))))

(event `ReportPuzzleSolving`
  (bind _nextpuzzle (`self.NextPuzzle`))
  (`/Engine/EditorBlueprintResources/StandardMacros.IsValid` _nextpuzzle
    (:`Is Valid`
      (`/Game/Development/Leonie_dump/Puzzles/BP_WeightPuzzle_001.Appear` _nextpuzzle)
      (`KismetSystemLibrary.PrintString` "Activate Next Puzzle!"))))

(fn `UserConstructionScript`)