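; BP_SinkableWater is a puzzle actor whose water sinks a set distance when activated.
; Activate fires once, playing a timeline that lerps the water down from the start position cached at BeginPlay.
; An EditInActivatedMode flag lets the construction script preview the sunken state in the editor, using paired DoOnce gates to avoid repeated offsets.
; BeginPlay undoes that preview offset before storing the start position.
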(event `self.ReceiveBeginPlay`
  (if (`self.EditInActivatedMode`)
    ;[1 1 1] Reset Editor Activate
    (`SceneComponent.K2_SetWorldLocation` (`self.water`) (`KismetMathLibrary.MakeVector` (.x (`SceneComponent.K2_GetComponentLocation` (`self.water`))) (.y (`SceneComponent.K2_GetComponentLocation` (`self.water`))) (+ (.z (`SceneComponent.K2_GetComponentLocation` (`self.water`))) (`self.SinkDownDistance`))) false false))
  ;[1 1 1] Set WorldPosition
  (set `self.StartPosition` (`SceneComponent.K2_GetComponentLocation` (`self.water`))))

(event `Activate`
  (bind _startposition (`self.StartPosition`))
  (`/Engine/EditorBlueprintResources/StandardMacros.DoOnce` false
    (:`Completed`
      (bind (_direction _sinkprogress) (`Timeline|SinkingWaterTime` :!via `PlayFromStart`)
        (:`Update`
          (`SceneComponent.K2_SetWorldLocation` (`self.water`) (`KismetMathLibrary.VLerp` _startposition (`KismetMathLibrary.MakeVector` (.x _startposition) (.y _startposition) (- (.z _startposition) (`self.SinkDownDistance`))) _sinkprogress) false false))))))

(fn `UserConstructionScript`
  (if (`self.EditInActivatedMode`)
    ;[1 1 1] Edit in ActivatedMode
    (`/Engine/EditorBlueprintResources/StandardMacros.DoOnce` false :!label _label
      (:`Completed`
        (`SceneComponent.K2_SetWorldLocation` (`self.water`) (`KismetMathLibrary.MakeVector` (.x (`SceneComponent.K2_GetComponentLocation` (`self.water`))) (.y (`SceneComponent.K2_GetComponentLocation` (`self.water`))) (- (.z (`SceneComponent.K2_GetComponentLocation` (`self.water`))) (`self.SinkDownDistance`))) false false)
        (goto _label_2 :!via `Reset`)))
    (else
      ;[1 1 1] Edit in DeactivatedMode
      (`/Engine/EditorBlueprintResources/StandardMacros.DoOnce` true :!label _label_2
        (:`Completed`
          (`SceneComponent.K2_SetWorldLocation` (`self.water`) (`KismetMathLibrary.MakeVector` (.x (`SceneComponent.K2_GetComponentLocation` (`self.water`))) (.y (`SceneComponent.K2_GetComponentLocation` (`self.water`))) (+ (.z (`SceneComponent.K2_GetComponentLocation` (`self.water`))) (`self.SinkDownDistance`))) false false)
          (goto _label :!via `Reset`))))))