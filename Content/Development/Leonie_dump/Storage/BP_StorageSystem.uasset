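; Storage container actor that the player opens with the pickup input inside its trigger sphere to move items to and from the inventory.
; Opening shows the storage widget, pauses the game and fills both panels from its StorageInventory map and the scene's single BP_InventorySystem.
; Clicked items switch sides based on PickupTime, which is zeroed in storage, then both panels refresh.
; Storage stacks items by name, and withdrawals require free inventory space.
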(event `self.ReceiveBeginPlay`
  ;[1 1 1] Initialize
  (`self.EnableInput` (`GameplayStatics.GetPlayerController` 0))
  (bind _outactors (`GameplayStatics.GetAllActorsOfClass` "/Game/Development/Leonie_dump/Inventory/BP_InventorySystem.BP_InventorySystem_C"))
  (if (== (`KismetArrayLibrary.Array_Length` _outactors) 1)
    (set `self.Inventory_System_Ref` (`|GetArrayItem` _outactors))
    (else
      (`KismetSystemLibrary.PrintString` "Storage System detected more or less than 1 Inventory System in scene!" true true (struct :`R` 1.0 :`B` 0.142592 :`A` 1.0) 10.0))))

(event `EnhancedInput|/Game/Development/Leonie_dump/Levels_dump/IA_Pickup`
  (params (ActionValue :type Boolean) (ElapsedSeconds :type "Float (double-precision)") (TriggeredSeconds :type "Float (double-precision)") (InputAction :type "InputAction Object Reference" :default "/Game/Development/Leonie_dump/Levels_dump/IA_Pickup.IA_Pickup"))
  ;[1 1 1] Open Storage
  (:`Completed`
    (if (`self.IsPlayerInRange`)
      (`self.OpenOrCloseStorage`))))

(event `OpenOrCloseStorage`
  (bind _returnvalue (`GameplayStatics.GetPlayerController` 0))
  ;[1 1 1] Open and close Inventory
  (`/Engine/EditorBlueprintResources/StandardMacros.IsValid` (`self.WB_Storage_Ref`)
    (:`Is Valid`
      (if (`Widget.IsVisible` (`self.WB_Storage_Ref`))
        (`GameplayStatics.SetGamePaused` false)
        (`KismetSystemLibrary.Delay` 0.1)
        (`Widget.RemoveFromParent` (`self.WB_Storage_Ref`))
        (`WidgetBlueprintLibrary.SetInputMode_GameOnly` _returnvalue)
        (set `PlayerController.bShowMouseCursor` false _returnvalue)
        (else
          (`UserWidget.AddToViewport` (stale _output_get) 0 :!label _label)
          (`WidgetBlueprintLibrary.SetInputMode_GameAndUIEx` (`GameplayStatics.GetPlayerController` 0) (`self.WB_Storage_Ref`) "DoNotLock" false)
          (set `PlayerController.bShowMouseCursor` true (`GameplayStatics.GetPlayerController` 0))
          (`GameplayStatics.SetGamePaused` true)
          (`/Game/Development/Leonie_dump/Storage/WBP_StorrageInterface.UpdateInventoryPannel` (`self.WB_Storage_Ref`) (`/Game/Development/Leonie_dump/Inventory/BP_InventorySystem.Inventory` (`self.Inventory_System_Ref`)) self)
          (`/Game/Development/Leonie_dump/Storage/WBP_StorrageInterface.UpdateStorage` (`self.WB_Storage_Ref`) (`self.StorageInventory`) self))))
    (:`Is Not Valid`
      (bind _returnvalue_2 (`|CreateWidget` "/Game/Development/Leonie_dump/Storage/WBP_StorrageInterface.WBP_StorrageInterface_C"))
      (bind _output_get (set `self.WB_Storage_Ref` _returnvalue_2))
      (goto _label))))

(event `self.TriggerSphere.OnComponentBeginOverlap`
  (params (OverlappedComponent :type "PrimitiveComponent Object Reference") (OtherActor :type "Actor Object Reference") (OtherComp :type "PrimitiveComponent Object Reference") (OtherBodyIndex :type Integer) (bFromSweep :type Boolean) (SweepResult :type "HitResult Structure (by ref)"))
  ;[1 1 1] Player Detection
  (cast `/Game/StarterContent/ThirdPerson/Blueprints/BP_ThirdPersonCharacter` OtherActor
    (:`then`
      (set `self.IsPlayerInRange` true))
    (:`CastFailed`
      (`KismetSystemLibrary.PrintString` "Something has triggered the Storage Trigger and is not a Player" true true (struct :`R` 1.0 :`B` 0.060141 :`A` 1.0)))))

(event `self.TriggerSphere.OnComponentEndOverlap`
  (params (OverlappedComponent :type "PrimitiveComponent Object Reference") (OtherActor :type "Actor Object Reference") (OtherComp :type "PrimitiveComponent Object Reference") (OtherBodyIndex :type Integer))
  ;[1 1 1] Player Detection
  (cast `/Game/StarterContent/ThirdPerson/Blueprints/BP_ThirdPersonCharacter` OtherActor
    (:`then`
      (set `self.IsPlayerInRange` false))
    (:`CastFailed`
      (`KismetSystemLibrary.PrintString` "Something has left the Storage Trigger and is not a Player" true true (struct :`R` 1.0 :`B` 0.060141 :`A` 1.0)))))

(event `ItemWasKlicked`
  (params (Item :type "/Game/Development/Leonie_dump/PickUps/S_ItemData Structure"))
  ;[1 1 1] Comment
  (`self.MoveItemBetwenLists` Item)
  ;;[1 1 1] UI Update
  (`/Game/Development/Leonie_dump/Storage/WBP_StorrageInterface.UpdateStorage` (`self.WB_Storage_Ref`) (`self.StorageInventory`) self)
  (`/Game/Development/Leonie_dump/Storage/WBP_StorrageInterface.UpdateInventoryPannel` (`self.WB_Storage_Ref`) (`/Game/Development/Leonie_dump/Inventory/BP_InventorySystem.Inventory` (`self.Inventory_System_Ref`)) self))

(fn `AddItemToStorage`
  (params (Item :type "/Game/Development/Leonie_dump/PickUps/S_ItemData Structure"))
  (bind _structout (setmembers `/Game/Development/Leonie_dump/PickUps/S_ItemData` :`StructRef` Item :`PickupTime` 0.0))
  (`BlueprintMapLibrary.Map_Add` (`self.StorageInventory`) (`KismetTextLibrary.Conv_TextToString` (`.Name_4_F8E0E59F4DED3ECE3D7832A06FFC4421` (break `/Game/Development/Leonie_dump/PickUps/S_ItemData` Item))) _structout))

(fn `DecreaseItem`
  (params (Item :type "/Game/Development/Leonie_dump/PickUps/S_ItemData Structure"))
  (locals (ItemName :type Text))
  (bind _value (`BlueprintMapLibrary.Map_Find` (`self.StorageInventory`) (`KismetTextLibrary.Conv_TextToString` (`local.ItemName`))))
  ;[1 1 1] Increase
  (set `local.ItemName` (`.Name_4_F8E0E59F4DED3ECE3D7832A06FFC4421` (break `/Game/Development/Leonie_dump/PickUps/S_ItemData` Item)))
  (bind _result (`/Engine/EditorBlueprintResources/StandardMacros.DecrementInt` (`.Amount_20_AC872A8743206116538ACDBA7E9D74CF` (break `/Game/Development/Leonie_dump/PickUps/S_ItemData` _value)))
    (:`  `
      (bind _structout (setmembers `/Game/Development/Leonie_dump/PickUps/S_ItemData` :`StructRef` _value :`Amount` _result))
      (`BlueprintMapLibrary.Map_Add` (`self.StorageInventory`) (`KismetTextLibrary.Conv_TextToString` (`local.ItemName`)) _structout))))

(fn `IncreaseAmount`
  (params (Item :type "/Game/Development/Leonie_dump/PickUps/S_ItemData Structure"))
  (locals (NewLocalVar :type Text))
  (bind _value (`BlueprintMapLibrary.Map_Find` (`self.StorageInventory`) (`KismetTextLibrary.Conv_TextToString` (`local.NewLocalVar`))))
  ;[1 1 1] Check ob Item wirklich im Storage ist
  (bind _returnvalue (`self.IsItemAlreadyInStorage` Item))
  (if _returnvalue
    ;[1 1 1] Increase
    (set `local.NewLocalVar` (`.Name_4_F8E0E59F4DED3ECE3D7832A06FFC4421` (break `/Game/Development/Leonie_dump/PickUps/S_ItemData` Item)))
    (bind _result (`/Engine/EditorBlueprintResources/StandardMacros.IncrementInt` (`.Amount_20_AC872A8743206116538ACDBA7E9D74CF` (break `/Game/Development/Leonie_dump/PickUps/S_ItemData` _value)))
      (:`  `
        (bind _structout (setmembers `/Game/Development/Leonie_dump/PickUps/S_ItemData` :`StructRef` _value :`Amount` _result))
        (`BlueprintMapLibrary.Map_Add` (`self.StorageInventory`) (`KismetTextLibrary.Conv_TextToString` (`local.NewLocalVar`)) _structout)
        (`KismetSystemLibrary.PrintString` "Increased")))
    (else
      ;[1 1 1] Debug
      (`KismetSystemLibrary.PrintString` (`KismetStringLibrary.Concat_StrStr` "Item with Key: " (`KismetTextLibrary.Conv_TextToString` (`local.NewLocalVar`)) " not found in Storage List!") true true (struct :`R` 1.0 :`B` 0.196138 :`A` 1.0) 10.0))))

(fn `IsItemAlreadyInStorage`
  (params (Item :type "/Game/Development/Leonie_dump/PickUps/S_ItemData Structure"))
  (returns (ReturnValue :type Boolean))
  (return (`BlueprintMapLibrary.Map_Contains` (`self.StorageInventory`) (`KismetTextLibrary.Conv_TextToString` (`.Name_4_F8E0E59F4DED3ECE3D7832A06FFC4421` (break `/Game/Development/Leonie_dump/PickUps/S_ItemData` Item))))))

(fn `MoveItemBetwenLists`
  (params (Item :type "/Game/Development/Leonie_dump/PickUps/S_ItemData Structure"))
  (locals (ItemToMove :type "/Game/Development/Leonie_dump/PickUps/S_ItemData Structure"))
  (bind (_name _image _weight _description _cathegory _value _amount _consumabletype _consumable_statvalue _consumable_energyvalue _pickuptime) (break `/Game/Development/Leonie_dump/PickUps/S_ItemData` (`local.ItemToMove`)))
  (bind _output_get (set `local.ItemToMove` Item))
  (if (> (`.PickupTime_23_72B68219414DE7AFB37B29B6206C8D61` (break `/Game/Development/Leonie_dump/PickUps/S_ItemData` _output_get)) 0.0)
    ;[1 1 1] Klicked Item is from Inventory
    ;;[0.5794 1 0.4828] Add item to Storage
    (`self.TryAddItem` (`local.ItemToMove`))
    ;;[1 0.4862 0.3355] Remove Item from Inventory
    (`/Game/Development/Leonie_dump/Inventory/BP_InventorySystem.TryRemoveItem` (`self.Inventory_System_Ref`) (`KismetStringLibrary.Concat_StrStr` (`KismetTextLibrary.Conv_TextToString` _name) (`KismetStringLibrary.Conv_DoubleToString` _pickuptime)))
    (else
      ;[1 1 1] Klicked Item is from Storage
      (bind _returnvalue (`/Game/Development/Leonie_dump/Inventory/BP_InventorySystem.IsEnoughSpaceInInventory` (`self.Inventory_System_Ref`)))
      (if _returnvalue
        ;;[1 0.5268 0.376] Remove item from Storage
        (`self.TryRemoveItem` (`local.ItemToMove`))
        ;;[0.5558 1 0.5477] Add Item to Inventory
        (`/Game/Development/Leonie_dump/Inventory/BP_InventorySystem.TryAddItem` (`self.Inventory_System_Ref`) (`local.ItemToMove`))
        (else
          (`KismetSystemLibrary.PrintString` "Inventory is full!"))))))

(fn `RemoveItem`
  (params (NewParam :type "/Game/Development/Leonie_dump/PickUps/S_ItemData Structure"))
  (`BlueprintMapLibrary.Map_Remove` (`self.StorageInventory`) (`KismetTextLibrary.Conv_TextToString` (`.Name_4_F8E0E59F4DED3ECE3D7832A06FFC4421` (break `/Game/Development/Leonie_dump/PickUps/S_ItemData` NewParam)))))

(fn `TryAddItem`
  (params (Item :type "/Game/Development/Leonie_dump/PickUps/S_ItemData Structure"))
  (bind _returnvalue (`self.IsItemAlreadyInStorage` Item))
  (if _returnvalue
    ;[1 1 1] Zähle den Item Amount hoch und update den Slot
    (`self.IncreaseAmount` Item)
    (else
      (`self.AddItemToStorage` Item))))

(fn `TryRemoveItem`
  (params (Item :type "/Game/Development/Leonie_dump/PickUps/S_ItemData Structure"))
  (if (> (`.Amount_20_AC872A8743206116538ACDBA7E9D74CF` (break `/Game/Development/Leonie_dump/PickUps/S_ItemData` Item)) 1)
    (`self.DecreaseItem` Item)
    (`KismetSystemLibrary.PrintString` "Decreased")
    (else
      (`self.RemoveItem` Item)
      (`KismetSystemLibrary.PrintString` "Remove"))))

(fn `UserConstructionScript`)