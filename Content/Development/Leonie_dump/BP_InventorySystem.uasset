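; Inventory system actor that stores picked-up items, tracks pickups in player range and toggles the inventory widget.
; The inventory input creates or reuses the widget, switching pause, cursor and input mode.
; TryAddItem timestamps pickup data and stores it in a map keyed by name plus pickup time.
; The duplicate check searches by name alone and only prints, never blocking the add; IncreaseItemAmount is an empty stub.
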(event `self.ReceiveBeginPlay`
  (`self.EnableInput` (`GameplayStatics.GetPlayerController` 0)))

(event `EnhancedInput|/Game/Development/Leonie_dump/Levels_dump/IA_Inventory`
  (params (ActionValue :type Boolean) (ElapsedSeconds :type "Float (double-precision)") (TriggeredSeconds :type "Float (double-precision)") (InputAction :type "InputAction Object Reference" :default "/Game/Development/Leonie_dump/Levels_dump/IA_Inventory.IA_Inventory"))
  (bind _returnvalue (`GameplayStatics.GetPlayerController` 0))
  ;[1 1 1] Open and close Inventory
  (:`Completed`
    (`/Engine/EditorBlueprintResources/StandardMacros.IsValid` (`self.WB_InventoryReference`)
      (:`Is Valid`
        (if (`Widget.IsVisible` (`self.WB_InventoryReference`))
          (`/Game/Development/Leonie_dump/WBP_InventoryWidget.PlayBlenoutAnimation` (`self.WB_InventoryReference`))
          (`GameplayStatics.SetGamePaused` false)
          (`KismetSystemLibrary.Delay` 0.1)
          (`Widget.RemoveFromParent` (`self.WB_InventoryReference`))
          (`WidgetBlueprintLibrary.SetInputMode_GameOnly` _returnvalue)
          (set `PlayerController.bShowMouseCursor` false _returnvalue)
          (else
            (`UserWidget.AddToViewport` (stale _output_get) 0 :!label _label)
            (`WidgetBlueprintLibrary.SetInputMode_GameAndUIEx` (`GameplayStatics.GetPlayerController` 0) (`self.WB_InventoryReference`) "DoNotLock" false)
            (set `PlayerController.bShowMouseCursor` true (`GameplayStatics.GetPlayerController` 0))
            (`GameplayStatics.SetGamePaused` true))))
      (:`Is Not Valid`
        (bind _returnvalue_2 (`|CreateWidget` "/Game/Development/Leonie_dump/WBP_InventoryWidget.WBP_InventoryWidget_C"))
        (bind _output_get (set `self.WB_InventoryReference` _returnvalue_2))
        (goto _label)))))

(event `ReportItemIsInRange`
  (params (NewItem :type "Actor Object Reference"))
  ;[1 1 1] Player reports a new Item in Range
  (`self.TryPercieveItem` NewItem))

(event `LogoutItemFromRange`
  (params (Item :type "Actor Object Reference"))
  ;[1 1 1] Player logs out an Item from Range
  (`self.TryRemoveItemFromPerceptionList` Item))

(fn `AddItemToInventory`
  (params (Item :type "/Game/Development/Leonie_dump/PickUps/S_ItemData Structure"))
  (bind (_name _image _weight _description _cathegory _value _amount _pickuptime) (break `/Game/Development/Leonie_dump/PickUps/S_ItemData` Item))
  (`BlueprintMapLibrary.Map_Add` (`self.Inventory`) (`KismetTextLibrary.Conv_TextToString` (`KismetTextLibrary.Conv_StringToText` (`KismetStringLibrary.Concat_StrStr` (`KismetTextLibrary.Conv_TextToString` _name) (`KismetStringLibrary.Conv_DoubleToString` _pickuptime)))) Item))

(fn `Increase Item Amount`)

(fn `IsTheItemAlreadyInTheInventory`
  (params (Item :type "/Game/Development/Leonie_dump/PickUps/S_ItemData Structure"))
  (returns (ReturnValue :type Boolean))
  ;[1 1 1] Gives a bool if a item is still in the Inventory
  (return (`BlueprintMapLibrary.Map_Contains` (`self.Inventory`) (`KismetTextLibrary.Conv_TextToString` (`.Name_4_F8E0E59F4DED3ECE3D7832A06FFC4421` (break `/Game/Development/Leonie_dump/PickUps/S_ItemData` Item))))))

(fn `TimestampPickupItem`
  (params (Item :type "/Game/Development/Leonie_dump/PickUps/S_ItemData Structure"))
  (returns (S_ItemData :type "/Game/Development/Leonie_dump/PickUps/S_ItemData Structure"))
  (bind (_name _image _weight _description _cathegory _value _amount) (break `/Game/Development/Leonie_dump/PickUps/S_ItemData` Item))
  (return (make `/Game/Development/Leonie_dump/PickUps/S_ItemData` _name _image _weight _description _cathegory _value _amount (`KismetSystemLibrary.GetGameTimeInSeconds`))))

(fn `TryAddItem`
  (params (Item :type "Actor Object Reference"))
  (returns (`Added?` :type Boolean))
  ;[1 1 1] Is it a Pickup Item?
  (bind _asbp_master_pickup_item (cast `/Game/Development/Leonie_dump/PickUps/BP_MasterPickupItem` Item)
    (:`then`
      (bind _output_get (set `self.currentItem` (`/Game/Development/Leonie_dump/PickUps/BP_MasterPickupItem.MyItemData` _asbp_master_pickup_item)))
      ;[1 1 1] Timestamp Pickup Item
      (bind _s_itemdata (`self.TimestampPickupItem` _output_get))
      (bind _output_get_2 (set `self.currentItem` _s_itemdata))
      ;[1 1 1] Add to Inventory
      (bind _returnvalue (`self.IsTheItemAlreadyInTheInventory` _output_get_2))
      (if _returnvalue
        (`KismetSystemLibrary.PrintString` "Object Stil exist in Inventory!"))
      (`self.AddItemToInventory` (`self.currentItem`))
      (`KismetSystemLibrary.PrintString` (`KismetStringLibrary.Concat_StrStr` "Added " (`KismetTextLibrary.Conv_TextToString` (`.Name_4_F8E0E59F4DED3ECE3D7832A06FFC4421` (break `/Game/Development/Leonie_dump/PickUps/S_ItemData` (`self.currentItem`))))))
      (`KismetSystemLibrary.PrintString` (`KismetStringLibrary.Concat_StrStr` "Inventory Count is " (`KismetStringLibrary.Conv_IntToString` (`BlueprintMapLibrary.Map_Length` (`self.Inventory`)))))
      (return true))
    (:`CastFailed`
      ;;[1 1 1] NEIN! Kein Pickup Item
      (set `self.currentItem` (struct)) ; Set to null if cast fails
      (`KismetSystemLibrary.PrintString` "Tried to Add an Actor to the Inventory that is not a pickup Item!" true true (struct :`R` 1.0 :`G` 0.011514 :`B` 0.141235 :`A` 1.0) 10.0)
      (return false))))

(fn `TryPercieveItem`
  (params (ItemInRange :type "Actor Object Reference"))
  (`KismetArrayLibrary.Array_Add` (`self.PickUpsInRange`) ItemInRange)
  (`KismetSystemLibrary.PrintString` (`KismetStringLibrary.Conv_IntToString` (`KismetArrayLibrary.Array_Length` (`self.PickUpsInRange`)))))

(fn `TryRemoveItemFromPerceptionList`
  (params (ItemToRemove :type "Actor Object Reference"))
  (bind _returnvalue (`KismetArrayLibrary.Array_Find` (`self.PickUpsInRange`) ItemToRemove))
  (if (>= _returnvalue 0)
    (`KismetArrayLibrary.Array_Remove` (`self.PickUpsInRange`) _returnvalue)
    (`KismetSystemLibrary.PrintString` "Item successful removed")
    (else
      (`KismetSystemLibrary.PrintString` "Item to remove not found!" true true (struct :`R` 1.0 :`B` 0.064177 :`A` 1.0) 10.0))))

(fn `UserConstructionScript`)