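; Experimental actor that prints snow tracks on the landscape beneath objects the player stands on.
; PrintSnowAtLocation runs a downward multi line trace against WorldStatic objects from the given location, with persistent debug drawing.
; A first hit on the landscape is left to the capture camera.
; Otherwise, it spawns NS_SnowPrintOnLandscape particles at each hit identified as landscape by HasHitLandscapeTag.
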(event `self.ReceiveTick`
  (params (DeltaSeconds :type "Float (single-precision)")))

(event `PrintSnowAtLocation`
  (params (Location :type "Vector Structure"))
  ;[1 1 1] Checke alle Hits die sich unter der Location befinden
  (bind _outhits (`KismetSystemLibrary.LineTraceMultiForObjects` :`Start` Location :`End` (`KismetMathLibrary.MakeVector` (.x Location) (.y Location) -1000.0) :`ObjectTypes` (`|MakeArray` "ObjectTypeQuery1" :!type "EObjectTypeQuery Enum") :`DrawDebugType` "Persistent"))
  ;[1 1 1] Wenn der erste Hit die Landscape ist passiert nix - da übernimmt die Capture Kamera die Spuren
  (if (not (`self.HasHitLandscapeTag` (`|GetArrayItem` _outhits)))
    ;[1 1 1] Wenn der Player auf einem Objekt steht, spawnen print partikel auf der Landscape unter dem Player
    (for _array_element _outhits
      (if (`self.HasHitLandscapeTag` _array_element)
        (`NiagaraFunctionLibrary.SpawnSystemAtLocation` "/Game/Development/Leonie_dump/Snow/Experimente/NS_SnowPrintOnLandscape.NS_SnowPrintOnLandscape" (`.Location` (`GameplayStatics.BreakHitResult` _array_element)))))))

(fn `UserConstructionScript`)