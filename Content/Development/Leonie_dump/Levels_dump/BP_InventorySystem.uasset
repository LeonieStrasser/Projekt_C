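; BP_InventorySystem is an actor that opens and closes the inventory screen on the IA_Inventory input; it holds no item logic.
; It enables player input on BeginPlay, creates WBP_InventoryWidget on first use and reuses the cached reference afterwards.
; Opening shows the widget with cursor and Game and UI input, then pauses the game.
; Closing unpauses, removes the widget and restores game-only input.
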(event `self.ReceiveBeginPlay`
  (`self.EnableInput` (`GameplayStatics.GetPlayerController` 0)))

(event `EnhancedInput|/Game/Development/Leonie_dump/Levels_dump/IA_Inventory`
  (params (ActionValue :type Boolean) (ElapsedSeconds :type "Float (double-precision)") (TriggeredSeconds :type "Float (double-precision)") (InputAction :type "InputAction Object Reference" :default "/Game/Development/Leonie_dump/Levels_dump/IA_Inventory.IA_Inventory"))
  (bind _returnvalue (`GameplayStatics.GetPlayerController` 0))
  (:`Completed`
    (`/Engine/EditorBlueprintResources/StandardMacros.IsValid` (`self.WB_InventoryReference`)
      (:`Is Valid`
        (if (`Widget.IsVisible` (`self.WB_InventoryReference`))
          (`GameplayStatics.SetGamePaused` false)
          (`Widget.RemoveFromParent` (`self.WB_InventoryReference`))
          (`WidgetBlueprintLibrary.SetInputMode_GameOnly` _returnvalue)
          (set `PlayerController.bShowMouseCursor` false _returnvalue)
          (else
            (`UserWidget.AddToViewport` (stale _output_get) 0 :!label _label)
            (`WidgetBlueprintLibrary.SetInputMode_GameAndUIEx` (`GameplayStatics.GetPlayerController` 0) (`self.WB_InventoryReference`) "DoNotLock" false)
            (set `PlayerController.bShowMouseCursor` true (`GameplayStatics.GetPlayerController` 0))
            (`GameplayStatics.SetGamePaused` true))))
      (:`Is Not Valid`
        (bind _returnvalue_2 (`|CreateWidget` "/Game/Development/Leonie_dump/Levels_dump/WBP_InventoryWidget.WBP_InventoryWidget_C"))
        (bind _output_get (set `self.WB_InventoryReference` _returnvalue_2))
        (goto _label)))))

(fn `UserConstructionScript`)