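; Actor that follows the player's mesh each tick and detects nearby water for drinking and wading.
; A box trace toggles the drink-hint widget and a placeholder debug print, while a line trace detects standing in water.
; Entering water lowers walk speed and reports coldness to BP_SurvivalManager; DoOnce gates reverse both on exit.
; Water is recognized by "water" in the hit actor's display name.
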(event `self.ReceiveBeginPlay`
  (bind _outactors (`GameplayStatics.GetAllActorsOfClass` "/Game/Development/Fea_dump/BP_SurvivalManager.BP_SurvivalManager_C"))
  (set `self.SurvivalManager_ref` (`|GetArrayItem` _outactors)))

(event `self.ReceiveTick`
  (params (DeltaSeconds :type "Float (single-precision)"))
  (bind _survivalmanager_ref (`self.SurvivalManager_ref`))
  (bind _charactermovement (`Character.CharacterMovement` (`GameplayStatics.GetPlayerCharacter` 0)))
  (bind _charactermovement_2 (`Character.CharacterMovement` (`GameplayStatics.GetPlayerCharacter` 0)))
  ;[1 1 1] set to player pos
  (`SceneComponent.K2_SetWorldTransform` (`self.DefaultSceneRoot`) (`SceneComponent.K2_GetComponentToWorld` (`Character.Mesh` (`GameplayStatics.GetPlayerCharacter` 0))) false false)
  (`|ExecutionSequence`
    (:`then_0`
      ;[1 1 1] check if player is near water to drink it
      (bind _outhit (`KismetSystemLibrary.BoxTraceSingle` (`SceneComponent.K2_GetComponentLocation` (`self.start point`)) (`SceneComponent.K2_GetComponentLocation` (`self.end point`)) (5.0 5.0 5.0) (struct) "TraceTypeQuery1"))
      (if (`KismetStringLibrary.Contains` (`KismetSystemLibrary.GetDisplayName` (`.HitActor` (`GameplayStatics.BreakHitResult` _outhit))) "water")
        (set `self.Player_is_looking_at_water` true)
        ;[1 1 1] placeholder UI
        (`KismetSystemLibrary.PrintString` "You can drink!")
        (`/Engine/EditorBlueprintResources/StandardMacros.DoOnce` false :!label _label
          (:`Completed`
            (bind _returnvalue (`|CreateWidget` "/Game/Development/Fea_dump/UI/WB_Drink_Hinweis.WB_Drink_Hinweis_C" (`GameplayStatics.GetPlayerController` 0)))
            (`UserWidget.AddToViewport` _returnvalue 0)))
        (else
          (set `self.Player_is_looking_at_water` false)
          (`Widget.RemoveFromParent` _returnvalue)
          (goto _label :!via `Reset`))))
    (:`then_1`
      (bind _outhit_2 (`KismetSystemLibrary.LineTraceSingle` (`SceneComponent.K2_GetComponentLocation` (`self.start point`)) (`SceneComponent.K2_GetComponentLocation` (`self.end point_2`)) "TraceTypeQuery1"))
      (if (`KismetStringLibrary.Contains` (`KismetSystemLibrary.GetDisplayName` (`.HitActor` (`GameplayStatics.BreakHitResult` _outhit_2))) "water")
        (set `self.Player_is_In_Water` true)
        (`/Engine/EditorBlueprintResources/StandardMacros.DoOnce` false :!label _label_2
          (:`Completed`
            (`/Game/Development/Fea_dump/BP_SurvivalManager.Report_Coldness` _survivalmanager_ref)
            (set `CharacterMovementComponent.MaxWalkSpeed` (- (`CharacterMovementComponent.MaxWalkSpeed` _charactermovement) (`self.InWater_walking_downgrade`)) _charactermovement)
            (goto _label_3 :!via `Reset`)))
        (else
          (set `self.Player_is_In_Water` false)
          (`/Engine/EditorBlueprintResources/StandardMacros.DoOnce` false :!label _label_3
            (:`Completed`
              (`/Game/Development/Fea_dump/BP_SurvivalManager.Report_noMoreColdness` _survivalmanager_ref)
              (set `CharacterMovementComponent.MaxWalkSpeed` (+ (`CharacterMovementComponent.MaxWalkSpeed` _charactermovement_2) (`self.InWater_walking_downgrade`)) _charactermovement_2)
              (goto _label_2 :!via `Reset`))))))))

(fn `UserConstructionScript`)