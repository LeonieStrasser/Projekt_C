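; BP_Storm_Border is a storm boundary that slows the player and makes them cold through two trigger zones.
; Cold_Zone overlaps toggle PlayerIsCold on the BP_SurvivalManager found at BeginPlay.
; While the player is in WindZone, Tick sets MaxWalkSpeed to their signed world X offset from FarthestPoint, so speed falls as that offset shrinks.
; Leaving WindZone stops the updates but does not restore walk speed.
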(event `self.ReceiveTick`
  (params (DeltaSeconds :type "Float (single-precision)"))
  (if (`self.Player_is_in_Windzone`)
    (`self.ApplyWindForce`)))

(event `self.ReceiveBeginPlay`
  (bind _outactors (`GameplayStatics.GetAllActorsOfClass` "/Game/Development/Fea_dump/BP_SurvivalManager.BP_SurvivalManager_C"))
  (set `self.SurvivalManager_ref` (`|GetArrayItem` _outactors)))

(event `self.Cold_Zone.OnComponentBeginOverlap`
  (params (OverlappedComponent :type "PrimitiveComponent Object Reference") (OtherActor :type "Actor Object Reference") (OtherComp :type "PrimitiveComponent Object Reference") (OtherBodyIndex :type Integer) (bFromSweep :type Boolean) (SweepResult :type "HitResult Structure (by ref)"))
  (cast `/Game/StarterContent/ThirdPerson/Blueprints/BP_ThirdPersonCharacter` OtherActor)
  (set `/Game/Development/Fea_dump/BP_SurvivalManager.Player_is_cold` true (`self.SurvivalManager_ref`)))

(event `self.Cold_Zone.OnComponentEndOverlap`
  (params (OverlappedComponent :type "PrimitiveComponent Object Reference") (OtherActor :type "Actor Object Reference") (OtherComp :type "PrimitiveComponent Object Reference") (OtherBodyIndex :type Integer))
  (cast `/Game/StarterContent/ThirdPerson/Blueprints/BP_ThirdPersonCharacter` OtherActor)
  (set `/Game/Development/Fea_dump/BP_SurvivalManager.Player_is_cold` false (`self.SurvivalManager_ref`)))

(event `ApplyWindForce`
  (bind _returnvalue_x (`KismetMathLibrary.BreakVector` (`SceneComponent.K2_GetComponentLocation` (`self.Farthest_point`))))
  (bind _returnvalue_x_2 (`KismetMathLibrary.BreakVector` (`SceneComponent.K2_GetComponentLocation` (`Character.CapsuleComponent` (`self.As BP Third Person Character`)))))
  (bind _output_get (set `self.Slow_down_amount` (- _returnvalue_x_2 _returnvalue_x)))
  (set `CharacterMovementComponent.MaxWalkSpeed` _output_get (`Character.CharacterMovement` (`self.As BP Third Person Character`))))

(event `self.WindZone.OnComponentBeginOverlap`
  (params (OverlappedComponent :type "PrimitiveComponent Object Reference") (OtherActor :type "Actor Object Reference") (OtherComp :type "PrimitiveComponent Object Reference") (OtherBodyIndex :type Integer) (bFromSweep :type Boolean) (SweepResult :type "HitResult Structure (by ref)"))
  (bind _asbp_third_person_character (cast `/Game/StarterContent/ThirdPerson/Blueprints/BP_ThirdPersonCharacter` OtherActor))
  (set `self.As BP Third Person Character` _asbp_third_person_character)
  (set `self.Player_is_in_Windzone` true))

(event `self.WindZone.OnComponentEndOverlap`
  (params (OverlappedComponent :type "PrimitiveComponent Object Reference") (OtherActor :type "Actor Object Reference") (OtherComp :type "PrimitiveComponent Object Reference") (OtherBodyIndex :type Integer))
  (cast `/Game/StarterContent/ThirdPerson/Blueprints/BP_ThirdPersonCharacter` OtherActor)
  (set `self.Player_is_in_Windzone` false))

(fn `UserConstructionScript`)