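; BP_Bed is a world bed that shows a prompt widget when the player character overlaps its collision and hides it when they leave.
; On overlap it asks the inventory system whether the player holds the bed upgrade item, then shows the upgrade or standard widget and records the result.
; BeginPlay finds the inventory and upgrade item data in the level, pre-creates both widgets and hides the UI, which turns toward the camera each tick.
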(event `self.collision.OnComponentBeginOverlap`
  (params (OverlappedComponent :type "PrimitiveComponent Object Reference") (OtherActor :type "Actor Object Reference") (OtherComp :type "PrimitiveComponent Object Reference") (OtherBodyIndex :type Integer) (bFromSweep :type Boolean) (SweepResult :type "HitResult Structure (by ref)"))
  (cast `/Game/StarterContent/ThirdPerson/Blueprints/BP_ThirdPersonCharacter` OtherActor)
  (set `self.Player_is_near_bed` true)
  (if true
    (bind _returnvalue (`/Game/Development/Leonie_dump/Inventory/BP_InventorySystem.FindItemByItsKey` (`self.Inventory_ref`) (`self.Upgrade_data`)))
    (if _returnvalue
      (`WidgetComponent.SetWidget` (`self.UI`) (stale `self.ReceiveBeginPlay` _returnvalue_2))
      (set `self.Player_has_BedUpgrade` true)
      (else
        (`WidgetComponent.SetWidget` (`self.UI`) (stale `self.ReceiveBeginPlay` _returnvalue))))
    (`SceneComponent.SetVisibility` (`self.UI`) true false)))

(event `self.collision.OnComponentEndOverlap`
  (params (OverlappedComponent :type "PrimitiveComponent Object Reference") (OtherActor :type "Actor Object Reference") (OtherComp :type "PrimitiveComponent Object Reference") (OtherBodyIndex :type Integer))
  (cast `/Game/StarterContent/ThirdPerson/Blueprints/BP_ThirdPersonCharacter` OtherActor)
  (set `self.Player_is_near_bed` false)
  (`SceneComponent.SetVisibility` (`self.UI`) false false :!label _label))

(event `self.ReceiveBeginPlay`
  (bind _outactors (`GameplayStatics.GetAllActorsOfClass` "/Game/Development/Leonie_dump/Inventory/BP_InventorySystem.BP_InventorySystem_C"))
  (set `self.Inventory_ref` (`|GetArrayItem` _outactors))
  (bind _outactors_2 (`GameplayStatics.GetAllActorsOfClass` "/Game/Development/Fea_dump/BP_Bed_Upgrade.BP_Bed_Upgrade_C"))
  (set `self.Upgrade_data` (`/Game/Development/Leonie_dump/PickUps/BP_MasterPickupItem.MyItemData` (`|GetArrayItem` _outactors_2)))
  (bind _returnvalue (`|CreateWidget` "/Game/Development/Fea_dump/UI/WB_Bed_UI.WB_Bed_UI_C"))
  (bind _returnvalue_2 (`|CreateWidget` "/Game/Development/Fea_dump/UI/WB_Bed_UI_upgrade.WB_Bed_UI_upgrade_C"))
  (goto _label))

(event `self.ReceiveTick`
  (params (DeltaSeconds :type "Float (single-precision)"))
  (bind _ui (`self.UI`))
  ;[1 1 1] make UI always face the player camera
  (`SceneComponent.K2_SetWorldRotation` _ui (`KismetMathLibrary.FindLookAtRotation` (`SceneComponent.K2_GetComponentLocation` _ui) (`SceneComponent.K2_GetComponentLocation` (`PlayerCameraManager.TransformComponent` (`GameplayStatics.GetPlayerCameraManager` 0)))) false false))

(fn `UserConstructionScript`)