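; Base area spawner that scatters a random number of Placeholder_item actors at random points inside its SpawnArea bounds.
; BeginPlay picks the target count from a min/max range, and Tick spawns one item per frame until it is reached.
; While the BP_SurvivalManager reports night, every Tick calls Reset, which destroys all Placeholder_item actors in the level, including other spawners', and rerolls the count.
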(event `self.ReceiveBeginPlay`
  (bind _outactors (`GameplayStatics.GetAllActorsOfClass` "/Game/Development/Fea_dump/BP_SurvivalManager.BP_SurvivalManager_C"))
  (set `self.survival_manager_ref` (`|GetArrayItem` _outactors))
  (set `self.Items_spawned` 0)
  (set `self.Items_to_be_spawned` (`KismetMathLibrary.RandomIntegerInRange` (`self.Min_spawn_amount`) (`self.Max_spawn_amount`))))

(event `self.ReceiveTick`
  (params (DeltaSeconds :type "Float (single-precision)"))
  (bind (_origin _boxextent) (`KismetSystemLibrary.GetComponentBounds` (`self.spawn_area`)))
  ;[1 1 1] spawning
  (if (`/Game/Development/Fea_dump/BP_SurvivalManager.At_night` (`self.survival_manager_ref`))
    (`self.Reset`))
  (if (not (== (`self.Items_spawned`) (`self.Items_to_be_spawned`)))
    (`|SpawnActorFromClass` "/Game/Development/Fea_dump/placeholder_item.placeholder_item_C" (`KismetMathLibrary.MakeTransform` (`KismetMathLibrary.RandomPointInBoundingBox` _origin _boxextent)) "Undefined" "MultiplyWithRoot" null null)
    (set `self.Items_spawned` (+ (`self.Items_spawned`) 1))))

(event `Reset`
  ;[1 1 1] remove all previously spawned items
  (bind _outactors (`GameplayStatics.GetAllActorsOfClass` "/Game/Development/Fea_dump/placeholder_item.placeholder_item_C"))
  (for _index (range (+ (`KismetArrayLibrary.Array_Length` _outactors) 1))
    (`self.K2_DestroyActor` (`|GetArrayItem` _outactors _index)))
  (set `self.Items_spawned` 0)
  (set `self.Items_to_be_spawned` (`KismetMathLibrary.RandomIntegerInRange` (`self.Min_spawn_amount`) (`self.Max_spawn_amount`))))

(fn `UserConstructionScript`)