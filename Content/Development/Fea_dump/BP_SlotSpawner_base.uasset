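; Base slot spawner that fills random child-component slots of its Mesh with a random number of SpawnItemClass actors.
; Tick spawns up to one item per frame until the target is met, tracking used transforms to avoid overlaps.
; Once full, night or player sleep reported by BP_SurvivalManager triggers a DoOnce-gated reset.
; The reset tallies surviving items, destroys them and rerolls the count, sometimes adding half that running tally.
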(event `self.ReceiveBeginPlay`
  (bind _outactors (`GameplayStatics.GetAllActorsOfClass` "/Game/Development/Fea_dump/BP_SurvivalManager.BP_SurvivalManager_C"))
  (set `self.survival_manager_ref` (`|GetArrayItem` _outactors))
  (set `self.Items_to_be_spawned` (`KismetMathLibrary.RandomIntegerInRange` (`self.Min_spawn_amount`) (`self.Max_spawn_amount`)))
  ;[1 1 1] add all slot transforms into the array
  (for _array_element (`SceneComponent.GetChildrenComponents` (`self.mesh`) false)
    (`KismetArrayLibrary.Array_Add` (`self.Transform_Array`) (`SceneComponent.K2_GetComponentToWorld` _array_element))
    (`KismetArrayLibrary.Array_Clear` (`self.spawned_items_array`))))

(event `self.ReceiveTick`
  (params (DeltaSeconds :type "Float (single-precision)"))
  (bind _survival_manager_ref (`self.survival_manager_ref`))
  (set `self.Items_spawned` (`KismetArrayLibrary.Array_Length` (`self.spawned_items_array`)))
  (if (== (`self.Items_spawned`) (`self.Items_to_be_spawned`))
    (`KismetArrayLibrary.Array_Clear` (`self.Transform_Array`))
    (if (or (`/Game/Development/Fea_dump/BP_SurvivalManager.At_night` _survival_manager_ref) (`/Game/Development/Fea_dump/BP_SurvivalManager.Player_just_slept` _survival_manager_ref))
      (`/Engine/EditorBlueprintResources/StandardMacros.DoOnce` false :!label _label
        (:`Completed`
          (`self.CheckHowManySlotsAreFull`)
          (`self.Reset`)))
      (else
        (goto _label :!via `Reset`)))
    (else
      ;[1 1 1] check that no Item spawns at the same location
      (`self.GetNewRandomTransform`)
      (if (`KismetArrayLibrary.Array_Contains` (`self.Control_transform_Array`) (`self.newTransform`))
        (`self.GetNewRandomTransform`)
        (else
          ;[1 1 1] spawning
          (bind _returnvalue (`|SpawnActorFromClass` (`self.SpawnItem_Class`) (`self.newTransform`) "Undefined" "MultiplyWithRoot" null null))
          (`KismetArrayLibrary.Array_Add` (`self.spawned_items_array`) _returnvalue)
          (set `self.Items_spawned` (+ (`self.Items_spawned`) 1))
          (`KismetArrayLibrary.Array_Add` (`self.Control_transform_Array`) (`self.newTransform`)))))))

(event `Reset`
  (bind _spawned_items_array (`self.spawned_items_array`))
  (bind _full_slot_amount (`self.Full_Slot_amount`))
  (bind _returnvalue (`KismetMathLibrary.RandomIntegerInRange` (`self.Min_spawn_amount`) (`self.Max_spawn_amount`)))
  ;[1 1 1] remove all previously spawned items
  (for _index (range (+ (`KismetArrayLibrary.Array_Length` _spawned_items_array) 1))
    (`self.K2_DestroyActor` (`|GetArrayItem` _spawned_items_array _index)))
  (if (> _returnvalue _full_slot_amount)
    (set `self.Items_to_be_spawned` _returnvalue)
    (else
      (set `self.Items_to_be_spawned` (+ _returnvalue (/ _full_slot_amount 2)))))
  ;[1 1 1] add all slot transforms into the array
  (for _array_element (`SceneComponent.GetChildrenComponents` (`self.mesh`) false)
    (`KismetArrayLibrary.Array_Add` (`self.Transform_Array`) (`SceneComponent.K2_GetComponentToWorld` _array_element))
    (`KismetArrayLibrary.Array_Clear` (`self.Control_transform_Array`))
    (`KismetArrayLibrary.Array_Clear` (`self.spawned_items_array`))
    (`KismetSystemLibrary.PrintString` "RESET")))

(event `GetNewRandomTransform`
  (set `self.newTransform` (`KismetArrayLibrary.Array_Random` (`self.Transform_Array`))))

(event `CheckHowManySlotsAreFull`
  (bind _spawned_items_array (`self.spawned_items_array`))
  (for _index (range (+ (`KismetArrayLibrary.Array_Length` _spawned_items_array) 1))
    (`/Engine/EditorBlueprintResources/StandardMacros.IsValid` (`|GetArrayItem` _spawned_items_array _index)
      (:`Is Valid`
        (set `self.Full_Slot_amount` (+ (`self.Full_Slot_amount`) 1)))
      (:`Is Not Valid`
        (set `self.Full_Slot_amount` (- (`self.Full_Slot_amount`) 1))))))

(fn `UserConstructionScript`)